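; BP_RayTraceCharacter is a character that fires a line trace along its forward vector when E is pressed.
; SingleLineTrace traces on the Visibility channel from the actor's location out to a configurable distance, with timed debug drawing.
; If the hit actor is a BP_RayHittable, it calls HitByRay with the impact point and an impulse scaled from the unnormalized trace vector.
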(event Input|KeyboardEvents|E
  (params (Key :type Key%20Structure))
  (:Pressed
    (CallFunction|SingleLineTrace)))

(fn ConstructionScript
  (|CallParentFunction))

(fn SingleLineTrace
  (bind _outhit (Collision|LineTraceByChannel (Transformation|GetActorLocation) (+ (* (Variables|Default|GetLineTraceDistaince) (Transformation|GetActorForwardVector)) (Transformation|GetActorLocation)) "TraceTypeQuery1" false 0 "ForDuration"))
  (bind _asbp_ray_hittable (Utilities|Casting|CastToBP_RayHittable (.hitactor _outhit)))
  (Default|HitbyRay _asbp_ray_hittable (.impactpoint _outhit) (* (- (.traceend _outhit) (.tracestart _outhit)) 2e+03)))